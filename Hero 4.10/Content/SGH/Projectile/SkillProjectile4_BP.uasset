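; Skill projectile that acts as a short-lived box damage area for the player's active skill.
; On BeginPlay it reads which of the four skills is in use, derives damage from attack power and the skill multiplier, and scales range from the skill struct.
; The box is sized and offset along X by that range.
; An overlap applies damage and destroys the box; the root component is destroyed after a half-second delay.
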(event EventBeginPlay
  (bind _playercharacter (Variables|Default|GetPlayerCharacter))
  (bind _range (Variables|Default|GetRange))
  (bind _box (Variables|Default|GetBox))
  (bind _relativelocation (Variables|/Script/Engine.SceneComponent|GetRelativeLocation _box))
  (bind (_x _y _z) (Math|Vector|BreakVector _relativelocation))
  (switch int (Variables|/Game/SGH/Character/PlayerCharacter/BP_FHero_Warrior.BP_FHero_Warrior_C|GetUsingSkill _playercharacter)
    (:1
      (Utilities|스킬기본값설정 _playercharacter (Variables|/Game/SGH/Character/PlayerCharacter/BP_FHero_Warrior.BP_FHero_Warrior_C|GetSkill1 _playercharacter)))
    (:2
      (Utilities|스킬기본값설정 _playercharacter (Variables|/Game/SGH/Character/PlayerCharacter/BP_FHero_Warrior.BP_FHero_Warrior_C|GetSkill2 _playercharacter)))
    (:3
      (Utilities|스킬기본값설정 _playercharacter (Variables|/Game/SGH/Character/PlayerCharacter/BP_FHero_Warrior.BP_FHero_Warrior_C|GetSkill3 _playercharacter)))
    (:4
      (Utilities|스킬기본값설정 _playercharacter (Variables|/Game/SGH/Character/PlayerCharacter/BP_FHero_Warrior.BP_FHero_Warrior_C|GetSkill4 _playercharacter))))
  (Components|Box|SetBoxExtent (Variables|Default|GetBox) (Math|Vector|MakeVector _range _range 4e+01) true)
  (Transformation|SetRelativeLocation _box (Math|Vector|MakeVector _range _y _z) false false)
  (Utilities|FlowControl|Delay 0.5)
  (Components|DestroyComponent (Variables|Default|GetDefaultSceneRoot)))

(event EventActorBeginOverlap
  (params (OtherActor :type Actor%20Object%20Reference))
  (Game|Damage|ApplyDamage OtherActor (Math|Conversions|ToFloat(Integer) (Variables|Default|GetDamage)) 0 0)
  (Components|DestroyComponent (Variables|Default|GetBox)))

(fn ConstructionScript)