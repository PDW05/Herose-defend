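; Skill projectile Blueprint that fires a beam with a growing damage box along local X.
; BeginPlay sets the beam end point to Range, then a delayed loop extends and shifts the box forward equally, keeping its rear edge fixed until MaxTime steps elapse.
; Overlapping actors receive Damage.
; Overlap, Hit or loop completion destroys the DefaultSceneRoot component rather than the actor.
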(event EventBeginPlay
  (bind _box (Variables|Default|GetBox))
  (bind _boxextent (Variables|/Script/Engine.BoxComponent|GetBoxExtent _box))
  (bind _relativelocation (Variables|/Script/Engine.SceneComponent|GetRelativeLocation _box))
  (bind (_x _y _z) (Math|Vector|BreakVector _relativelocation))
  (bind (_x_2 _y_2 _z_2) (Math|Vector|BreakVector _boxextent))
  (Variables|Default|Settime 0)
  (Class|ParticleSystemComponent|SetBeamEndPoint (Variables|Default|GetParticleSystem) 1 (Math|Vector|MakeVector (Variables|Default|GetRange) 0.0 0.0))
  (Components|Box|SetBoxExtent _box (Math|Vector|MakeVector (+ _x_2 5e+01) _y_2 _z_2) true :!label _label)
  (Transformation|SetRelativeLocation _box (Math|Vector|MakeVector (+ _x 5e+01) _y _z) false false)
  (Utilities|FlowControl|Delay 0.1)
  (bind _output_get (Variables|Default|Settime (+ (Variables|Default|Gettime) 1)))
  (if (< _output_get (Variables|Default|GetMaxTime))
    (goto _label)
    (else
      (Components|DestroyComponent (Variables|Default|GetDefaultSceneRoot)))))

(event EventActorBeginOverlap
  (params (OtherActor :type Actor%20Object%20Reference))
  (Game|Damage|ApplyDamage OtherActor (Math|Conversions|ToFloat(Integer) (Variables|Default|GetDamage)) 0 0)
  (Components|DestroyComponent (Variables|Default|GetDefaultSceneRoot)))

(event Collision|EventHit
  (params (MyComp :type Primitive%20Component%20Object%20Reference) (Other :type Actor%20Object%20Reference) (OtherComp :type Primitive%20Component%20Object%20Reference) (bSelfMoved :type Boolean) (HitLocation :type Vector :default "0, 0, 0") (HitNormal :type Vector :default "0, 0, 0") (NormalImpulse :type Vector :default "0, 0, 0") (Hit :type Hit%20Result%20Structure%20%28by%20ref%29))
  (Components|DestroyComponent (Variables|Default|GetDefaultSceneRoot)))

(fn ConstructionScript)