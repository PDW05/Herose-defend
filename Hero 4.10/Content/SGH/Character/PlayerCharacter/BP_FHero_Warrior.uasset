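; Warrior hero player character that moves relative to the camera's yaw and fires a ranged projectile with the A key.
; Arrow keys set direction flags, which GetRotation turns into one of eight yaw angles from the control rotation, defaulting to forward.
; The attack spawns Projectile_BP ahead of the character along that rotation.
; AttackAnimation then plays the same slash montage on the main mesh and each modular armor and body mesh.
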(event EventBeginPlay
  (Variables|Default|SetHealth 100))

(event Input|AxisEvents|InputAxisMoveForward
  (params (AxisValue :type Float%20%28single-precision%29))
  ;[1 1 1] 이동
  (Pawn|Input|AddMovementInput (Math|Vector|GetForwardVector (Math|Rotator|MakeRotator 0.0 0.0 (.Yaw (Math|Rotator|BreakRotator (Pawn|GetControlRotation :!class /Script/Engine.Pawn))))) AxisValue false))

(event Input|AxisEvents|InputAxisMoveRight
  (params (AxisValue :type Float%20%28single-precision%29))
  ;[1 1 1] 이동
  (Pawn|Input|AddMovementInput (Math|Vector|GetRightVector (Math|Rotator|MakeRotator 0.0 0.0 (.Yaw (Math|Rotator|BreakRotator (Pawn|GetControlRotation :!class /Script/Engine.Pawn))))) AxisValue false))

(event Input|KeyboardEvents|Right
  (params (Key :type Key%20Structure :default "AnyKey"))
  (:Pressed
    (Variables|Default|SetRight true))
  (:Released
    (Variables|Default|SetRight false)))

(event Input|KeyboardEvents|A
  (params (Key :type Key%20Structure :default "AnyKey"))
  ;[1 1 1] 원거리 공격
  (:Pressed
    (bind _rotation (CallFunction|GetRotation (Variables|Default|GetLeft) (Variables|Default|GetRight) (Variables|Default|GetForward) (Variables|Default|GetBackward) (Pawn|GetControlRotation :!class /Script/Engine.Pawn)))
    (Game|SpawnActorfromClass "/Game/SGH/Projectile/Projectile_BP.Projectile_BP_C" (Math|Transform|MakeTransform (+ (Transformation|GetActorLocation) (* (Math|Vector|GetForwardVector _rotation) 1e+02)) _rotation) "AlwaysSpawn" (Components|GetOwner) 0)
    (CallFunction|AttackAnimation)))

(event Input|KeyboardEvents|Left
  (params (Key :type Key%20Structure :default "AnyKey"))
  (:Pressed
    (Variables|Default|SetLeft true))
  (:Released
    (Variables|Default|SetLeft false)))

(event Input|KeyboardEvents|Down
  (params (Key :type Key%20Structure :default "AnyKey"))
  (:Pressed
    (Variables|Default|SetBackward true))
  (:Released
    (Variables|Default|SetBackward false)))

(event Input|KeyboardEvents|Up
  (params (Key :type Key%20Structure :default "AnyKey"))
  (:Pressed
    (Variables|Default|SetForward true))
  (:Released
    (Variables|Default|SetForward false)))

(fn ConstructionScript)

(fn GetRotation
  (params (Left :type Boolean) (Right :type Boolean) (Forward :type Boolean) (Backward :type Boolean) (getRotation :type Rotator))
  (bind _yaw (Math|Rotator|BreakRotator getRotation))
  (if (and Left Forward) ; 왼쪽 앞
    (return (Math|Rotator|MakeRotator 0.0 0.0 (- _yaw 45.0)))
    (elif (and Right Forward) ; 오른쪽 앞
      (return (Math|Rotator|MakeRotator 0.0 0.0 (+ _yaw 45.0)))
      (elif (and Left Backward) ; 왼쪽 뒤
        (return (Math|Rotator|MakeRotator 0.0 0.0 (- _yaw 135.0)))
        (elif (and Right Backward) ; 오른쪽 뒤
          (return (Math|Rotator|MakeRotator 0.0 0.0 (+ _yaw 135.0)))
          (else
            (if Forward ; 앞
              _
              (elif Left ; 왼쪽
                (return (Math|Rotator|MakeRotator 0.0 0.0 (- _yaw 9e+01)))
                (elif Right ; 오른쪽
                  (return (Math|Rotator|MakeRotator 0.0 0.0 (+ _yaw 9e+01)))
                  (elif Backward ; 뒤
                    (return (Math|Rotator|MakeRotator 0.0 0.0 (+ _yaw 1.8e+02)))
                    (else
                      _)))))
            (return (Math|Rotator|MakeRotator 0.0 0.0 _yaw))))))))

(fn AttackAnimation
  (Animation|Montage|MontagePlay (Components|SkeletalMesh|GetAnimInstance (Variables|Default|GetChest_Armor_B_02_SkelMesh)) "/Game/SGH/Character/PlayerCharacter/SlashAttack_Anim_Montage.SlashAttack_Anim_Montage" 1.0)
  (Animation|Montage|MontagePlay (Components|SkeletalMesh|GetAnimInstance (Variables|Default|GetAcc_leg_SkelMesh)) "/Game/SGH/Character/PlayerCharacter/SlashAttack_Anim_Montage.SlashAttack_Anim_Montage" 1.0)
  (Animation|Montage|MontagePlay (Components|SkeletalMesh|GetAnimInstance (Variables|Default|GetBoots_A_SkelMesh)) "/Game/SGH/Character/PlayerCharacter/SlashAttack_Anim_Montage.SlashAttack_Anim_Montage" 1.0)
  (Animation|Montage|MontagePlay (Components|SkeletalMesh|GetAnimInstance (Variables|Default|GetGlove_A_Left_SkelMesh)) "/Game/SGH/Character/PlayerCharacter/SlashAttack_Anim_Montage.SlashAttack_Anim_Montage" 1.0)
  (Animation|Montage|MontagePlay (Components|SkeletalMesh|GetAnimInstance (Variables|Default|GetGlove_A_Right_SkelMesh)) "/Game/SGH/Character/PlayerCharacter/SlashAttack_Anim_Montage.SlashAttack_Anim_Montage" 1.0)
  (Animation|Montage|MontagePlay (Components|SkeletalMesh|GetAnimInstance (Variables|Default|Getears02_SkelMesh)) "/Game/SGH/Character/PlayerCharacter/SlashAttack_Anim_Montage.SlashAttack_Anim_Montage" 1.0)
  (Animation|Montage|MontagePlay (Components|SkeletalMesh|GetAnimInstance (Variables|Default|GetHair_04_SkelMesh)) "/Game/SGH/Character/PlayerCharacter/SlashAttack_Anim_Montage.SlashAttack_Anim_Montage" 1.0)
  (Animation|Montage|MontagePlay (Components|SkeletalMesh|GetAnimInstance (Variables|Default|GetHelmet_B_01_SkelMesh)) "/Game/SGH/Character/PlayerCharacter/SlashAttack_Anim_Montage.SlashAttack_Anim_Montage" 1.0)
  (Animation|Montage|MontagePlay (Components|SkeletalMesh|GetAnimInstance (Variables|Default|GetShorts_D_SkelMesh)) "/Game/SGH/Character/PlayerCharacter/SlashAttack_Anim_Montage.SlashAttack_Anim_Montage" 1.0)
  (Animation|Montage|MontagePlay (Components|SkeletalMesh|GetAnimInstance (Variables|Default|GetShoulder_B_Left_SkelMesh)) "/Game/SGH/Character/PlayerCharacter/SlashAttack_Anim_Montage.SlashAttack_Anim_Montage" 1.0)
  (Animation|Montage|MontagePlay (Components|SkeletalMesh|GetAnimInstance (Variables|Default|GetShoulder_B_Right_SkelMesh)) "/Game/SGH/Character/PlayerCharacter/SlashAttack_Anim_Montage.SlashAttack_Anim_Montage" 1.0)
  (Animation|Montage|MontagePlay (Components|SkeletalMesh|GetAnimInstance (Variables|Character|GetMesh)) "/Game/SGH/Character/PlayerCharacter/SlashAttack_Anim_Montage.SlashAttack_Anim_Montage" 1.0))