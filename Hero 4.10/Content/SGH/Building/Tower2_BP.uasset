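; Tower2 building Blueprint that sets its health on BeginPlay and contains logic to fire Projectile_BP on a cooldown.
; Tick accumulates elapsed seconds, then enters a Gate that has no open or close triggers wired.
; The Gate's exit compares that time to the last attack plus cooldown, spawns the projectile at the tower's own transform and records the attack time.
; No targeting or damage handling is present.
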(event EventBeginPlay
  (Variables|Default|SetHealth 100))

(event EventTick
  (params (DeltaSeconds :type Float%20%28single-precision%29))
  (Utilities|FlowControl|Sequence
    (:then_0
      (Variables|Default|SetTimeSecond (+ (* DeltaSeconds 1.0) (Variables|Default|GetTimeSecond))))
    (:then_1
      (Utilities|FlowControl|Gate true
        (:Exit
          (Utilities|FlowControl|Sequence
            (:then_1
              (if (<= (+ (Variables|Default|GetAttackCooltime) (Variables|Default|GetLastAttackTime)) (Variables|Default|GetTimeSecond))
                (Game|SpawnActorfromClass "/Game/SGH/Projectile/Projectile_BP.Projectile_BP_C" (Transformation|GetActorTransform) "Undefined" 0 0)
                (Variables|Default|SetLastAttackTime (Variables|Default|GetTimeSecond))))))))))

(fn ConstructionScript
  (|CallParentFunction))